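; Back door Blueprint that starts open and slides shut, optionally triggering a level unload behind it.
; BeginPlay moves the Cube to its open height and caches the FPSCharacter.
; CloseDoor plays OpenDoorTimeline to lerp the Cube's Z to the closed position, then calls CallUnloadLevel on the player with LevelToUnload if ShouldUnloadLevel is set.
; OpenDoor has no live logic, only an unconnected delayed destroy.
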(event Custom|CloseDoor
  (bind _doorslidingtrack (Timeline|OpenDoorTimeline Play)
    (:Update
      (Transformation|SetRelativeLocation (Variables|Default|GetCube) (Math|Vector|MakeVector 0.0 0.0 (Math|Float|Lerp (Variables|Default|GetDoorOpenPosition) (Variables|Default|GetDoorClosedPosition) _doorslidingtrack)) false false))
    (:Finished
      (if (Variables|Default|GetShouldUnloadLevel)
        (Default|CallUnloadLevel (Variables|Default|GetPlayerRef) (Variables|Default|GetLevelToUnload))))))

(event EventBeginPlay
  (Transformation|SetRelativeLocation (Variables|Default|GetCube) (Math|Vector|MakeVector 0.0 0.0 (Variables|Default|GetDoorOpenPosition)) false false)
  (bind _returnvalue (Actor|GetActorOfClass "/Game/Blueprints/Player/FPS-Character.FPS-Character_C"))
  (Variables|Default|SetPlayerRef _returnvalue))

(event EventTick
  (params (DeltaSeconds :type Float%20%28single-precision%29)))

(fn ConstructionScript)