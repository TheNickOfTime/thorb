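; Door actor that gates progress behind a minigame and slides open when the player wins it.
; It binds to FPS-Character events that toggle its BP_Interact_UI prompt: available when the minigame is offered, unavailable on a loss.
; Interact has the player load the chosen minigame version and disables the prompt.
; A win loads the configured level, slides the Cube on Z via a timeline with door sounds, then destroys the actor.
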(event OnComponentActivated(BP_Interact_UI)
  (params (Component :type Actor%20Component%20Object%20Reference) (bReset :type Boolean))
  (bind _asbp_interact_ui (Utilities|Casting|CastToBP_Interact_UI Component))
  (Default|Initialize _asbp_interact_ui (Variables|Default|GetInteractSprite) (Variables|Default|GetInteractSpriteContainer) self))

(event Custom|OnWinMinigame
  (Default|CallLoadLevel (Variables|Default|GetPlayerRef) (Variables|Default|GetLevelToLoad))
  (Audio|Components|Audio|FadeIn (Variables|Default|GetSFX_mini_game_door_open) 0.3 0.5 0.0 "Linear" :!class /Script/Engine.AudioComponent)
  (bind _doorslidingtrack (Timeline|OpenDoorTimeline Play)
    (:Update
      (Transformation|SetRelativeLocation (Variables|Default|GetCube) (Math|Vector|MakeVector 0.0 0.0 (Math|Float|Lerp (Variables|Default|GetDoorClosedPosition) (Variables|Default|GetDoorOpenPosition) _doorslidingtrack)) false false))
    (:Finished
      (Audio|Components|Audio|FadeOut (Variables|Default|GetSFX_mini_game_door_open) 0.5 0.0 "Linear" :!class /Script/Engine.AudioComponent)
      (Audio|Components|Audio|FadeIn (Variables|Default|GetSFX_Heavy_door_close_1) 0.0 0.4 0.0 "Linear" :!class /Script/Engine.AudioComponent)
      (Utilities|FlowControl|Delay 2.0)
      (Actor|DestroyActor))))

(event Custom|OnMakeMinigameAvailable
  (Default|MakeAvailable (Variables|Default|GetBP_Interact_UI)))

(event Custom|OnLoseMinigame
  (Default|MakeUnavailable (Variables|Default|GetBP_Interact_UI)))

(event EventBeginPlay
  (bind _asfps_character (Utilities|Casting|CastToFPS-Character (Game|GetPlayerCharacter 0)))
  (bind _output_get (Variables|Default|SetPlayerRef _asfps_character))
  (EventDispatchers|BindEventtoMakeMinigameAvailable _output_get (delegate Custom|OnMakeMinigameAvailable))
  (EventDispatchers|BindEventtoLoseMinigame _output_get (delegate Custom|OnLoseMinigame))
  (EventDispatchers|BindEventtoWinMinigame _output_get (delegate Custom|OnWinMinigame)))

(event EventTick
  (params (DeltaSeconds :type Float%20%28single-precision%29)))

(event Input|ActionEvents|InputActionInteract
  (params (Key :type Key%20Structure :default "None"))
  (:Pressed
    (Default|CallLoadMinigameLevel (Variables|Default|GetPlayerRef) (Variables|Default|GetMinigameVersion))
    (Default|MakeUnavailable (Variables|Default|GetBP_Interact_UI))))

(fn ConstructionScript)