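; ShotgunBlast is a projectile actor representing a shotgun blast that damages enemy characters.
; A size alpha sets its lifespan, end scale and initial projectile speed; the cone grows each tick until the lifespan ends and it destroys itself.
; On overlap with an enemy, it traces from the spawn point to arrows tagged HitCheck, dealing damage once at the first unobstructed one, so cover blocks the blast.
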(event OnComponentBeginOverlap(Cone)
  (params (OverlappedComponent :type Primitive%20Component%20Object%20Reference) (OtherActor :type Actor%20Object%20Reference) (OtherComp :type Primitive%20Component%20Object%20Reference) (OtherBodyIndex :type Integer) (bFromSweep :type Boolean) (SweepResult :type Hit%20Result%20Structure%20%28by%20ref%29))
  (bind _asenemy__character (Utilities|Casting|CastToEnemy-Character OtherActor))
  (bind _array_element (Utilities|Array|ForEachLoopwithBreak (Actor|GetComponentsbyTag _asenemy__character "/Script/Engine.ArrowComponent" "HitCheck") :!label _label)
    (:LoopBody
      (bind _returnvalue (Collision|LineTraceByChannel (Variables|Default|GetStartLocation) (Transformation|GetWorldLocation _array_element) "TraceTypeQuery5" false 0 "None"))
      (if (not _returnvalue)
        (Default|TakeDamage _asenemy__character 1e+02)
        (goto _label Break)))))

(event EventBeginPlay
  (Variables|Default|SetLifeTimer 0.0)
  (Variables|Default|SetLifeSpan (Math|Float|Lerp (Variables|Default|GetLowLifeSpan) (Variables|Default|GetHighLifeSpan) (Variables|Default|GetSizeOfBlastAlpha)))
  (Variables|Default|SetEndSize (Math|Vector|Lerp(Vector) (Variables|Default|GetSmallEndSize) (Variables|Default|GetLargeEndSize) (Variables|Default|GetSizeOfBlastAlpha)))
  (Variables|Default|SetStartLocation (Transformation|GetActorLocation)))

(event EventTick
  (params (DeltaSeconds :type Float%20%28single-precision%29))
  (if (>= (Variables|Default|GetLifeTimer) (Variables|Default|GetLifeSpan))
    (Actor|DestroyActor)
    (else
      (Variables|Default|SetLifeTimer (+ (Variables|Default|GetLifeTimer) DeltaSeconds))
      (Transformation|SetActorRelativeScale3D (Math|Vector|Lerp(Vector) (Variables|Default|GetStartSize) (Variables|Default|GetEndSize) (/ (Variables|Default|GetLifeTimer) (Variables|Default|GetLifeSpan)))))))

(fn ConstructionScript
  (Variables|/Script/Engine.ProjectileMovementComponent|SetInitialSpeed (Variables|Default|GetProjectileMovement) (Math|Float|Lerp (Variables|Default|GetLowVelocity) (Variables|Default|GetHighVelocity) (Variables|Default|GetSizeOfBlastAlpha))))