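; ShotgunTester is a test actor that fires ShotgunBlast actors at another ShotgunTester instance.
; On BeginPlay it searches all instances, stores non-shooters as Target (the last found wins) and starts a looping Shoot timer.
; Each timer tick, instances flagged IsShooter print a debug message and spawn a blast at their root, rotated toward Target with full blast size.
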(event Custom|Shoot
  (bind _defaultsceneroot (Variables|Default|GetDefaultSceneRoot))
  (bind _returnvalue (Transformation|GetWorldLocation _defaultsceneroot))
  (if (Variables|Default|GetIsShooter)
    (Development|PrintString "Hello")
    (Game|SpawnActorfromClass "/Game/Blueprints/Player/ShotgunBlast.ShotgunBlast_C" (Math|Transform|MakeTransform _returnvalue (Math|Rotator|FindLookatRotation _returnvalue (Transformation|GetWorldLocation (Variables|ShotgunTester_C|GetDefaultSceneRoot (Variables|Default|GetTarget))))) "Undefined" 0 1.0 0)))

(event EventBeginPlay
  (bind _outactors (Actor|GetAllActorsOfClass "ShotgunTester_C"))
  (for _array_element _outactors
    (if (not (Variables|ShotgunTester_C|GetIsShooter _array_element))
      (Variables|Default|SetTarget _array_element)
      (Utilities|Time|SetTimerbyEvent (delegate Custom|Shoot) 1.0 true))))

(event Collision|EventActorBeginOverlap
  (params (OtherActor :type Actor%20Object%20Reference)))

(event EventTick
  (params (DeltaSeconds :type Float%20%28single-precision%29)))

(fn ConstructionScript)