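; Interaction trigger that lets the FPS character enter and leave a minigame by pressing Enter while overlapping it.
; Overlap enables input on the actor and stores the player; leaving disables it.
; Entering starts a non-blocking level stream, immediately finds a ResurrectPlayer to possess through FPS-Controller, and turns on minigame view.
; Exiting unloads the level, repossesses the stored player and turns the view off.
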(event Custom|LoadMinigame
  (Class|GameplayStatics|LoadStreamLevelbySoftObjectPtr (Variables|Default|GetLevelToStream) true false)
  (bind _returnvalue (Actor|GetActorOfClass "/Game/Blueprints/Minigame/Resurrect/Resurrect-Player.Resurrect-Player_C"))
  (Default|PossessMinigameCharacter (.AsFPS-Controller (Utilities|Casting|CastToFPS-Controller (Game|GetPlayerController 0))) _returnvalue)
  (Default|CallSetMinigameViewon (Variables|Default|GetPlayer)))

(event Custom|UnloadMinigame
  (Class|GameplayStatics|UnloadStreamLevelbySoftObjectPtr (Variables|Default|GetLevelToStream) false)
  (Default|PossessMinigameCharacter (.AsFPS-Controller (Utilities|Casting|CastToFPS-Controller (Game|GetPlayerController 0))) (Variables|Default|GetPlayer))
  (Default|CallSetMinigameViewOff (Variables|Default|GetPlayer)))

(event Collision|EventActorBeginOverlap
  (params (OtherActor :type Actor%20Object%20Reference))
  (bind _asfps_character (Utilities|Casting|CastToFPS-Character OtherActor))
  (Variables|Default|SetPlayer _asfps_character)
  (Variables|Default|SetIsIn true)
  (Input|EnableInput (Game|GetPlayerController 0))
  (Development|PrintString "Hello"))

(event Collision|EventActorEndOverlap
  (params (OtherActor :type Actor%20Object%20Reference))
  (Utilities|Casting|CastToFPS-Character OtherActor)
  (Variables|Default|SetIsIn false)
  (Input|DisableInput (Game|GetPlayerController 0)))

(event Input|KeyboardEvents|Enter
  (params (Key :type Key%20Structure :default "None"))
  (:Pressed
    (if (Variables|Default|GetIsIn)
      (bind _output_get (Variables|Default|SetInMinigame (not (Variables|Default|GetInMinigame))))
      (if _output_get
        (CallFunction|LoadMinigame)
        (else
          (CallFunction|UnloadMinigame))))))

(fn ConstructionScript)