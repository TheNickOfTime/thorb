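; BP-Dialogue-Trigger-Volume is a trigger actor that unlocks a scripted dialogue when the player's FPS-Character overlaps it.
; It caches the player character on BeginPlay.
; On overlap by an FPS-Character, it waits for a configurable delay, then sets the TriggerCondition of the player's ScriptedDialogues entry at DialogueIndex to true.
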(event EventBeginPlay
  (bind _asfps_character (Utilities|Casting|CastToFPS-Character (Game|GetPlayerCharacter 0)))
  (Variables|Default|SetPlayerRef _asfps_character))

(event Collision|EventActorBeginOverlap
  (params (OtherActor :type Actor%20Object%20Reference))
  (Utilities|Casting|CastToFPS-Character OtherActor)
  (Utilities|FlowControl|Delay (Variables|Default|GetDelay))
  (|SetBy-RefVar (.TriggerCondition (Utilities|Struct|BreakDialogue (Utilities|Array|Get(acopy) (Variables|/Game/Blueprints/Player/FPS-Character.FPS-Character_C|GetScriptedDialogues (Variables|Default|GetPlayerRef)) (Variables|Default|GetDialogueIndex)))) true))

(event EventTick
  (params (DeltaSeconds :type Float%20%28single-precision%29)))

(fn ConstructionScript)