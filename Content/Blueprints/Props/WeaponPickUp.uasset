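; Weapon pickup prop that hovers on looping up/down timelines, with an interact prompt rotated toward the player every tick.
; On Interact, it stops floating, disables player input and ramps the sphere's glow through a timeline whose event tracks spawn a hidden teleporter and trigger level loading.
; When finished, it calls empty unlock and weapon-state functions, restores input, reveals the teleporter and hides the pickup.
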(event OnComponentActivated(BP_Interact_UI)
  (params (Component :type Actor%20Component%20Object%20Reference) (bReset :type Boolean))
  (bind _asbp_interact_ui (Utilities|Casting|CastToBP_Interact_UI Component))
  (Default|Initialize _asbp_interact_ui (Variables|Default|GetInteractSprite) (Variables|Default|GetSpriteContainer) self))

(event Custom|Play%20FloatUp
  (bind _hovercurve (Timeline|FloatUp PlayFromStart)
    (:Update
      (Transformation|SetRelativeLocation (Variables|Default|GetSphere) (Math|Vector|Lerp(Vector) (Variables|Default|GetLowHoverLocation) (Variables|Default|GetHighHoverLocation) _hovercurve) false false))
    (:Finished
      (Variables|Default|SetIsGoingUp false)
      (CallFunction|PlayFloatDown))))

(event Custom|Play%20FloatDown
  (bind _hovercurve (Timeline|FloatDown PlayFromStart)
    (:Update
      (Transformation|SetRelativeLocation (Variables|Default|GetSphere) (Math|Vector|Lerp(Vector) (Variables|Default|GetHighHoverLocation) (Variables|Default|GetLowHoverLocation) _hovercurve) false false))
    (:Finished
      (Variables|Default|SetIsGoingUp true)
      (CallFunction|PlayFloatUp))))

(event Custom|StopFloating
  (if (Variables|Default|GetIsGoingUp)
    (bind _hovercurve (Timeline|FloatUp Stop)
      (:Update
        (Transformation|SetRelativeLocation (Variables|Default|GetSphere) (Math|Vector|Lerp(Vector) (Variables|Default|GetLowHoverLocation) (Variables|Default|GetHighHoverLocation) _hovercurve) false false))
      (:Finished
        (Variables|Default|SetIsGoingUp false)
        (CallFunction|PlayFloatDown)))
    (else
      (bind _hovercurve_2 (Timeline|FloatDown Stop)
        (:Update
          (Transformation|SetRelativeLocation (Variables|Default|GetSphere) (Math|Vector|Lerp(Vector) (Variables|Default|GetHighHoverLocation) (Variables|Default|GetLowHoverLocation) _hovercurve_2) false false))
        (:Finished
          (Variables|Default|SetIsGoingUp true)
          (CallFunction|PlayFloatUp))))))

(event EventBeginPlay
  (bind _returnvalue (Actor|GetActorOfClass "/Game/Blueprints/Player/FPS-Character.FPS-Character_C"))
  (Variables|Default|SetPlayer _returnvalue)
  (bind _returnvalue_2 (Rendering|Material|CreateDynamicMaterialInstance (Variables|Default|GetSphere) 0 0 "None" :!class /Script/Engine.PrimitiveComponent))
  (bind _output_get (Variables|Default|SetGlowingMaterial _returnvalue_2))
  (bind _returnvalue_3 (Rendering|Material|GetScalarParameterValue _output_get "Brightness" :!class /Script/Engine.MaterialInstanceDynamic))
  (Variables|Default|SetInitialBrightness _returnvalue_3)
  (CallFunction|PlayFloatUp))

(event EventTick
  (params (DeltaSeconds :type Float%20%28single-precision%29))
  (CallFunction|FaceInteracttoPlayer)
  (if (Variables|Default|GetIsGoingUp)
    _))

(event Input|ActionEvents|InputActionInteract
  (params (Key :type Key%20Structure :default "None"))
  (bind _sphere (Variables|Default|GetSphere))
  (:Pressed
    (Audio|PlaySoundatLocation "/Game/Audio/Orb/SFX_Weapon_pickup_charge.SFX_Weapon_pickup_charge" (Transformation|GetActorLocation) "0, 0, 0" 1.0 1.0 1.0 0 0 0)
    (Audio|Components|Audio|FadeOut (Variables|Default|GetSFX_weapon_pickup_idle) 2.0 0.0 "Linear" :!class /Script/Engine.AudioComponent)
    (Default|MakeUnavailable (Variables|Default|GetBP_Interact_UI))
    (Input|DisableInput (Variables|Default|GetPlayer) (Game|GetPlayerController 0))
    (CallFunction|StopFloating)
    (bind _brightness (Timeline|CollectWeapon PlayFromStart)
      (:Update
        (Rendering|Material|SetScalarParameterValue (Variables|Default|GetGlowingMaterial) "Brightness" (Math|Float|Lerp (Variables|Default|GetInitialBrightness) (Variables|Default|GetFinalBrightness) _brightness) :!class /Script/Engine.MaterialInstanceDynamic))
      (:Finished
        (CallFunction|UnlockPlayerWeapon)
        (CallFunction|ChangePlayerWeaponState)
        (Input|EnableInput (Variables|Default|GetPlayer) (Game|GetPlayerController 0))
        (Default|SetVisibility (Variables|Default|GetTeleporterRef) true)
        (Rendering|SetVisibility (Variables|Default|GetPointLight) false false)
        (Rendering|SetVisibility _sphere false false)
        (Collision|SetCollisionEnabled _sphere "NoCollision")
        (Audio|PlaySoundatLocation "/Game/Audio/Orb/Cues/SFX_pickup.SFX_pickup" "0, 0, 0" "0, 0, 0" 1.0 1.0 0.0 0 0 0))
      (:SpawnTeleporter
        (bind _returnvalue (Game|SpawnActorfromClass "/Game/Test/Levi/Teleporter.Teleporter_C" (Transformation|GetWorldTransform (Variables|Default|GetTeleporterSpawn)) "Undefined" 0 (Variables|Default|GetTeleportTransform) false 0))
        (Variables|Default|SetTeleporterRef _returnvalue))
      (:LoadLevel
        (Default|CallLoadLevel (Variables|Default|GetPlayer) (Variables|Default|GetLevelToLoad))))))

(fn ConstructionScript)

(fn UnlockPlayerWeapon)

(fn ChangePlayerWeaponState)

(fn FaceInteracttoPlayer
  (bind _spritecontainer (Variables|Default|GetSpriteContainer))
  (Transformation|SetWorldRotation _spritecontainer (Math|Rotator|FindLookatRotation (Transformation|GetWorldLocation _spritecontainer) (Transformation|GetActorLocation (Variables|Default|GetPlayer))) false false))