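; Siren prop that signals when a minigame is available by showing two spotlights and bulbs and spinning its cylinder.
; On BeginPlay it finds the FPSCharacter and binds to its minigame-available and level-load events, which set the Available and Unavailable states.
; A small state machine with start, tick and end hooks toggles the lights, rotates the cylinder a fixed step per frame while available, and resets its rotation when unavailable.
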(event Custom|OnMakeMinigameAvailable
  (CallFunction|SwitchMinigameState "NewEnumerator1"))

(event Custom|OnLoadMinigameLevel
  (params (MinigameVersion :type Integer))
  (CallFunction|SwitchMinigameState "NewEnumerator0"))

(event EventBeginPlay
  (bind _returnvalue (Actor|GetActorOfClass "/Game/Blueprints/Player/FPS-Character.FPS-Character_C"))
  (bind _output_get (Variables|Default|SetPlayerRef _returnvalue))
  (EventDispatchers|BindEventtoMakeMinigameAvailable _output_get (delegate Custom|OnMakeMinigameAvailable))
  (EventDispatchers|BindEventtoLoadMinigameLevel _output_get (delegate Custom|OnLoadMinigameLevel)))

(event Collision|EventActorBeginOverlap
  (params (OtherActor :type Actor%20Object%20Reference)))

(event EventTick
  (params (DeltaSeconds :type Float%20%28single-precision%29))
  (CallFunction|OnMinigameStateTick (Variables|Default|GetMinigameState)))

(event Custom|OnMinigameStateTick
  (params (State :type MinigameState%20Enum :default "NewEnumerator0"))
  (switch Utilities|FlowControl|Switch|SwitchonMinigameState State
    (:NewEnumerator1
      (CallFunction|AvailableTick))))

(event Custom|OnMinigameStateStart
  (params (New%20State :type MinigameState%20Enum :default "NewEnumerator0"))
  (switch Utilities|FlowControl|Switch|SwitchonMinigameState New%20State
    (:NewEnumerator0
      (CallFunction|UnavailableStart))
    (:NewEnumerator1
      (CallFunction|AvailableStart))))

(event Custom|OnMinigameStateEnd
  (params (Old%20State :type MinigameState%20Enum :default "NewEnumerator0"))
  (switch Utilities|FlowControl|Switch|SwitchonMinigameState Old%20State))

(event Custom|SwitchMinigameState
  (params (NewState :type MinigameState%20Enum :default "NewEnumerator0"))
  ;[1 1 1] Switch State
  (if (Utilities|Enum|NotEqual(Enum) NewState (Variables|Default|GetMinigameState))
    (CallFunction|OnMinigameStateEnd (Variables|Default|GetMinigameState))
    (Variables|Default|SetMinigameState NewState)
    (CallFunction|OnMinigameStateStart NewState)))

(event Custom|AvailableStart
  (Rendering|SetVisibility (Variables|Default|GetSpotLight) true false)
  (Rendering|SetVisibility (Variables|Default|GetSpotLight1) true false)
  (Rendering|SetVisibility (Variables|Default|GetBulbs) true false))

(event Custom|UnavailableStart
  (Transformation|SetRelativeRotation (Variables|Default|GetCylinder) "0, 0, 0" false false)
  (Rendering|SetVisibility (Variables|Default|GetSpotLight) false false)
  (Rendering|SetVisibility (Variables|Default|GetSpotLight1) false false)
  (Rendering|SetVisibility (Variables|Default|GetBulbs) false false))

(event Custom|AvailableTick
  (Transformation|AddRelativeRotation (Variables|Default|GetCylinder) "0, 0,-3.000000" false false))

(fn ConstructionScript)