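; Health pickup actor that restores health to an overlapping FPS-Character, then destroys itself.
; Tick accumulates a lifetime timer and, once it reaches the blink-out start time, starts the BlinkOut timeline a single time.
; The timeline's Blink event toggles the heart particle system's visibility, and the actor is destroyed when the timeline finishes.
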(event EventBeginPlay)

(event Collision|EventActorBeginOverlap
  (params (OtherActor :type Actor%20Object%20Reference))
  (bind _asfps_character (Utilities|Casting|CastToFPS-Character OtherActor))
  (Default|RegainHealth _asfps_character (Variables|Default|GetHealthToRegain))
  (Actor|DestroyActor))

(event EventTick
  (params (DeltaSeconds :type Float%20%28single-precision%29))
  (bind _output_get (Variables|Default|SetLifeTimer (+ (Variables|Default|GetLifeTimer) DeltaSeconds)))
  (if (not (Variables|Default|GetIsBlinkingOut))
    (if (>= _output_get (Variables|Default|GetBlinkingOutStartTime))
      (Variables|Default|SetIsBlinkingOut true)
      (Timeline|BlinkOut Play
        (:Finished
          (Actor|DestroyActor))
        (:Blink
          (Rendering|SetVisibility (Variables|Default|GetHeartParticleSystem) (not (Variables|/Script/Engine.SceneComponent|GetbVisible (Variables|Default|GetHeartParticleSystem))) false))))))

(fn ConstructionScript)