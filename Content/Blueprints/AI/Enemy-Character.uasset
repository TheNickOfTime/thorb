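; Enemy character: a floating orb drawn with Paper2D sprites that faces the player and can shoot projectiles at the player camera.
; Tick bobs sprite and sphere along a spline, picks left, right or front eye sprites from a lagged look vector, and applies continuous laser damage.
; Damage triggers a red flicker; death notifies the player, may drop a health pickup and removes it from EnemyManager.
; BeginPlay randomises size and animation phase.
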(event Custom|SetLaserDamage
  (params (IsTakingDamage? :type Boolean))
  (Variables|Default|SetIsBeingDamagedByLaser IsTakingDamage?))

(event Custom|StartDamageFlicker
  (Timeline|GetDamaged PlayFromStart
    (:MakeRed
      (Sprite|SetSpriteColor (Variables|Default|GetPaperSprite) (Variables|Default|GetRedColor)))
    (:MakeNormal
      (Sprite|SetSpriteColor (Variables|Default|GetPaperSprite) (Variables|Default|GetNormalColor)))))

(event EventTick
  (params (DeltaSeconds :type Float%20%28single-precision%29))
  (bind _returnvalue (Transformation|GetActorLocation))
  (bind _playerref (Variables|Default|GetPlayerRef))
  (bind _returnvalue_2 (Transformation|GetActorLocation _playerref))
  (Transformation|SetActorRotation (Math|Rotator|FindLookatRotation (Math|Vector|MakeVector (.x _returnvalue) (.y _returnvalue) 0.0) (Math|Vector|MakeVector (.x _returnvalue_2) (.y _returnvalue_2) 0.0)))
  (CallFunction|FloatingMovement)
  (CallFunction|LerpLookDirection)
  (if (Variables|Default|GetIsBeingDamagedByLaser)
    (CallFunction|TakeDamage (* (Variables|Default|GetLaserDamagePerSec) (Utilities|Time|GetWorldDeltaSeconds)))))

(event EventBeginPlay
  (bind _asfps_character (Utilities|Casting|CastToFPS-Character (Game|GetPlayerCharacter 0)))
  (Variables|Default|SetPlayerRef _asfps_character)
  (Variables|Default|SetHealth (Variables|Default|GetMaxHealth))
  (Default|CallEnemySpawn self)
  (CallFunction|SetRandomPlaybackPos)
  (CallFunction|SetEnemySize)
  (Development|PrintString (Utilities|String|Append "Health: " (Utilities|String|ToString(Float) (Variables|Default|GetHealth))) true true "(R=0.000000,G=0.660000,B=1.000000,A=1.000000)" 1e+01))

(fn ConstructionScript
  (Variables|/Script/Engine.CharacterMovementComponent|SetMaxWalkSpeed (Variables|Character|GetCharacterMovement) (Variables|_Parameters|GetMoveSpeed)))

(fn Shoot
  (bind _papersprite (Variables|Default|GetPaperSprite))
  (bind _returnvalue (Transformation|GetWorldLocation _papersprite))
  (Game|SpawnActorfromClass "/Game/Blueprints/AI/BP_Enemy_Projectile.BP_Enemy_Projectile_C" (Math|Transform|MakeTransform _returnvalue (Math|Rotator|FindLookatRotation _returnvalue (Transformation|GetWorldLocation (Variables|/Game/Blueprints/Player/FPS-Character.FPS-Character_C|GetCamera (Variables|Default|GetPlayerRef))))) "Undefined" 0 0))

(fn Stopshot)

(fn TakeDamage
  (params (Damage :type Float%20%28single-precision%29))
  (bind _returnvalue (Pawn|GetController))
  (bind _asenemy__controller (Utilities|Casting|CastToEnemy-Controller _returnvalue))
  (Development|PrintString (Utilities|String|Append "Starting HP: " (Utilities|String|ToString(Float) (Variables|Default|GetHealth))) true true "(R=0.000000,G=0.660000,B=1.000000,A=1.000000)" 1e+01)
  (bind _output_get (Variables|Default|SetHealth (- (Variables|Default|GetHealth) Damage)))
  (Development|PrintString (Utilities|String|Append "New HP: " (Utilities|String|ToString(Float) (Variables|Default|GetHealth))) true true "(R=0.000000,G=0.660000,B=1.000000,A=1.000000)" 1e+01)
  (CallFunction|StartDamageFlicker)
  (if (<= _output_get 0.0)
    (Default|CallEnemyDeath (Variables|Default|GetPlayerRef))
    (CallFunction|TrytoSpawnHealthPickup)
    (Audio|SpawnSoundatLocation "/Game/Audio/Vox/Cues/VOX_Enemy_death.VOX_Enemy_death" (Transformation|GetActorLocation) "0, 0, 0" 0.8 1.0 0.0 0 0)
    (Default|RemoveEnemy (Variables|/Game/Blueprints/Player/FPS-Character.FPS-Character_C|GetEnemyManager (Variables|Default|GetPlayerRef)) (Utilities|Struct|MakeEnemyManagerData self (Variables|/Game/Blueprints/AI/Enemy-Controller.Enemy-Controller_C|GetPlayerDistance _asenemy__controller) (Variables|/Game/Blueprints/AI/Enemy-Controller.Enemy-Controller_C|GetCanAttack _asenemy__controller)))
    (Actor|DestroyActor)))

(fn FloatingMovement
  (bind _minfloattime (Variables|Default|GetMinFloatTime))
  (bind _maxfloattime (Variables|Default|GetMaxFloatTime))
  (bind _output_get (Variables|Default|SetFloatTime (Math|Float|Clamp(Float) (+ (Variables|Default|GetFloatTime) (* (Utilities|Time|GetWorldDeltaSeconds) (Math|Float|SelectFloat 1.0 -1.0 (Variables|Default|GetFloatDirection)) (Variables|Default|GetFloatSpeed))) _minfloattime _maxfloattime)))
  (Variables|Default|SetFloatDirection (select (or (>= _output_get _maxfloattime) (<= _output_get _minfloattime)) (not (Variables|Default|GetFloatDirection)) (Variables|Default|GetFloatDirection)))
  (Transformation|SetRelativeLocation (Variables|Default|GetPaperSprite) (Spline|GetLocationatTime (Variables|Default|GetSpline) _output_get "Local" false) false false)
  (Transformation|SetRelativeLocation (Variables|Default|GetSphere) (Spline|GetLocationatTime (Variables|Default|GetSpline) _output_get "Local" false) false false))

(fn TakeLaserDamage
  (bind _output_get (Variables|Default|SetHealth (Math|Float|Clamp(Float) (- (Variables|Default|GetHealth) (* (Utilities|Time|GetWorldDeltaSeconds) (Variables|Default|GetLaserDamagePerSec))) 0.0 (Variables|Default|GetMaxHealth))))
  (Development|PrintString (Utilities|String|ToString(Float) _output_get)))

(fn TrytoSpawnHealthPickup
  (if (<= (Math|Random|RandomFloat) (Variables|Default|GetChanceOfHealthSpawn))
    (Game|SpawnActorfromClass "/Game/Blueprints/AI/Health-Pickup.Health-Pickup_C" (Math|Transform|MakeTransform (Transformation|GetWorldLocation (Variables|Default|GetPaperSprite))) "Undefined" 0 0)))

(fn LerpLookDirection
  (bind _returnvalue (Transformation|GetActorForwardVector))
  (bind _output_get (Variables|Default|SetLookDirection (Math|Vector|Lerp(Vector) (Variables|Default|GetLookDirection) _returnvalue (* (Utilities|Time|GetWorldDeltaSeconds) (Variables|Default|GetLookSpeed)))))
  (Rendering|Components|Sprite|SetSprite (Variables|Default|GetPaperSprite) (select (> (Math|Float|Absolute(Float) (Class|LowEntryExtendedStandardLibrary|RoundDecimals (- (Class|KismetMathLibrary|DegAcos (.z (Math|Vector|CrossProduct (- _returnvalue _output_get) _returnvalue))) 9e+01) 2)) (Variables|Default|GetLookDeadZone)) (select (> (Class|LowEntryExtendedStandardLibrary|RoundDecimals (- (Class|KismetMathLibrary|DegAcos (.z (Math|Vector|CrossProduct (- _returnvalue _output_get) _returnvalue))) 9e+01) 2) 0.0) "/Game/Art/Enemy-Main/enemyOrbEyeLeft_Sprite.enemyOrbEyeLeft_Sprite" "/Game/Art/Enemy-Main/enemyOrbEyeRight_Sprite.enemyOrbEyeRight_Sprite") "/Game/Art/Enemy-Main/enemyOrbEyeFront_Sprite.enemyOrbEyeFront_Sprite")))

(fn SetEnemySize
  (bind _size (Variables|Default|GetSize))
  (bind _sphere (Variables|Default|GetSphere))
  (bind _output_get (Variables|Default|SetCurrentSize (Math|Random|RandomFloatinRange (.current _size) (.max _size))))
  (Transformation|SetRelativeScale3D (Variables|Default|GetPaperSprite) (Math|Vector|MakeVector _output_get _output_get _output_get))
  (Components|Sphere|SetSphereRadius _sphere (* _output_get (Variables|/Script/Engine.SphereComponent|GetSphereRadius _sphere)) true)
  (Transformation|SetRelativeScale3D (Variables|Default|GetDecal) (Math|Vector|MakeVector 1.0 _output_get _output_get)))

(fn SetRandomPlaybackPos
  (bind _floating_rocks (Variables|Default|GetFloating%20rocks))
  (bind _returnvalue (Class|PaperFlipbookComponent|GetFlipbookLengthinFrames _floating_rocks))
  (bind _returnvalue_2 (Math|Random|RandomIntegerinRange 0 _returnvalue))
  (Class|PaperFlipbookComponent|SetPlaybackPositioninFrames (Variables|Default|GetFloating%20rocks) _returnvalue_2 false)
  (Class|PaperFlipbookComponent|SetPlaybackPositioninFrames (Variables|Default|GetFloating%20rocks1) _returnvalue_2 false)
  (Variables|Default|SetFloatTime (Math|Random|RandomFloatinRange (Variables|Default|GetMinFloatTime) (Variables|Default|GetMaxFloatTime))))