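; Enemy manager component that lets only the enemies nearest its owner attack, capped at MaxActive.
; On BeginPlay it gathers all EnemyCharacter actors into a struct array of enemy, distance and active flag.
; Each Tick it updates distances, flags entries matching the smallest sorted values, then writes distance and CanAttack to each Enemy-Controller.
; Helper functions handle enemy removal and debug text.
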(event EventBeginPlay
  (CallFunction|ResetEnemyList))

(event EventTick
  (params (DeltaSeconds :type Float%20%28single-precision%29))
  (CallFunction|UpdateDistances)
  (CallFunction|CompareDistances)
  (CallFunction|SetEnemyVariables))

(fn ResetEnemyList
  (Utilities|Array|Clear (Variables|Default|GetData))
  (bind _outactors (Actor|GetAllActorsOfClass "/Game/Blueprints/AI/Enemy-Character.Enemy-Character_C"))
  (for _array_element _outactors
    (Utilities|Array|Add (Variables|Default|GetData) (Utilities|Struct|MakeEnemyManagerData _array_element 0.0 false))))

(fn UpdateDistances
  (for (_array_element _array_index) (Variables|Default|GetData)
    (bind _structout (Utilities|Struct|SetmembersinEnemyManagerData _array_element (Math|Vector|Distance(Vector) (Transformation|GetActorLocation (.Enemy (Utilities|Struct|BreakEnemyManagerData _array_element))) (Transformation|GetActorLocation (Components|GetOwner)))))
    (Utilities|Array|SetArrayElem (Variables|Default|GetData) _array_index _structout)))

(fn CompareDistances
  (bind _floats (LocalVariables|GetFloats))
  (for _array_element (Variables|Default|GetData)
    (Utilities|Array|Add _floats (.distance _array_element)))
  (Class|LowEntryExtendedStandardLibrary|SortFloatArrayDirectly _floats false)
  (Utilities|Array|Resize (LocalVariables|GetFloats) (Variables|Default|GetMaxActive))
  (for (_array_element_2 _array_index) (Variables|Default|GetData)
    (bind _structout (Utilities|Struct|SetmembersinEnemyManagerData _array_element_2 (Utilities|Array|ContainsItem (LocalVariables|GetFloats) (.Distance (Utilities|Struct|BreakEnemyManagerData _array_element_2)))))
    (Utilities|Array|SetArrayElem (Variables|Default|GetData) _array_index _structout)))

(fn DatatoString
  (LocalVariables|SetDebugText "")
  (for _array_element (Variables|Default|GetData)
    (bind _output_get (LocalVariables|SetDebugText (Utilities|String|Append (LocalVariables|GetDebugText) " 
" (Utilities|GetDisplayName (.enemy _array_element)) ", " (Utilities|String|ToString(Float) (.distance _array_element)) ", " (Utilities|String|ToString(Boolean) (.active _array_element)))))
    (return _output_get)))

(fn SetEnemyVariables
  (for _array_element (Variables|Default|GetData)
    (bind _asenemy__controller (Utilities|Casting|CastToEnemy-Controller (AI|GetAIController (.enemy _array_element))))
    (Variables|/Game/Blueprints/AI/Enemy-Controller.Enemy-Controller_C|SetPlayerDistance _asenemy__controller (.distance _array_element))
    (Variables|/Game/Blueprints/AI/Enemy-Controller.Enemy-Controller_C|SetCanAttack _asenemy__controller (.active _array_element))))

(fn RemoveEnemy
  (params (Enemy :type Enemy%20Manager%20Data%20Structure))
  (Utilities|Array|RemoveItem (Variables|Default|GetData) Enemy))