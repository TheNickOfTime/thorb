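; Enemy1 is a basic enemy actor that fires projectiles and dies when its health runs out.
; The startshoot event spawns a BP_Enemytemp_Projectile at the capsule's transform, while stopshoot calls an empty Stopshot function.
; When a capsule overlap ends and a BP_Enemytemp_Projectile, the same class it fires, still overlaps, it subtracts DamageTaken from Health and destroys itself at zero or below.
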(event OnComponentEndOverlap(CapsuleComponent)
  (params (OverlappedComponent :type Primitive%20Component%20Object%20Reference) (OtherActor :type Actor%20Object%20Reference) (OtherComp :type Primitive%20Component%20Object%20Reference) (OtherBodyIndex :type Integer))
  (Utilities|IsValid (Utilities|Array|Get(acopy) (Collision|GetOverlappingActors (Variables|Collision|GetCapsuleComponent) "/Game/Test/Victoria/BP_Enemytemp_Projectile.BP_Enemytemp_Projectile_C" :!class /Script/Engine.PrimitiveComponent))
    (:Is%20Valid
      (Development|PrintString "Enemy get hit")
      (CallFunction|TakeDamage))))

(event Custom|startshoot
  (CallFunction|Shoot)
  (Development|PrintString "enemy shoot")
  (Utilities|FlowControl|Delay 3.0))

(event Custom|stopshoot
  (CallFunction|Stopshot))

(fn ConstructionScript)

(fn Shoot
  (Game|SpawnActorfromClass "/Game/Test/Victoria/BP_Enemytemp_Projectile.BP_Enemytemp_Projectile_C" (Transformation|GetWorldTransform (Variables|Collision|GetCapsuleComponent)) "Undefined" 0 0))

(fn Stopshot)

(fn TakeDamage
  (bind _output_get (Variables|Default|SetHealth (- (Variables|Default|GetHealth) (Variables|Default|GetDamage%20Taken))))
  (if (<= _output_get 0.0)
    (Actor|DestroyActor)))