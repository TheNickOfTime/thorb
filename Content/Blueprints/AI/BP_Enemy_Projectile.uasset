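; BP_Enemy_Projectile is an enemy projectile actor with a sphere mesh and a humming orb sound.
; On BeginPlay it fades in the hum and starts a timed delay that destroys the actor when it expires.
; Actor Hit and SphereMesh component hit share one path that prints the struck component's name, then destroys the projectile after a zero-length delay.
; The graph applies no damage.
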(event OnComponentHit(SphereMesh)
  (params (HitComponent :type Primitive%20Component%20Object%20Reference) (OtherActor :type Actor%20Object%20Reference) (OtherComp :type Primitive%20Component%20Object%20Reference) (NormalImpulse :type Vector :default "0, 0, 0") (Hit :type Hit%20Result%20Structure%20%28by%20ref%29))
  (Development|PrintString (Utilities|String|Append "Enemy shot " (Utilities|GetDisplayName (stale Collision|EventHit OtherComp))) true true "(R=0.602283,G=0.835775,B=1.000000,A=1.000000)")
  (Utilities|FlowControl|Delay 0.0)
  (Actor|DestroyActor))

(event EventBeginPlay
  (Audio|Components|Audio|FadeIn (Variables|Default|GetSFX_orb_hum) 0.1 1.0 0.0 "Linear" :!class /Script/Engine.AudioComponent)
  (Utilities|FlowControl|Delay 2e+01)
  (Actor|DestroyActor))

(event Collision|EventHit
  (params (MyComp :type Primitive%20Component%20Object%20Reference) (Other :type Actor%20Object%20Reference) (OtherComp :type Primitive%20Component%20Object%20Reference) (bSelfMoved :type Boolean) (HitLocation :type Vector :default "0, 0, 0") (HitNormal :type Vector :default "0, 0, 0") (NormalImpulse :type Vector :default "0, 0, 0") (Hit :type Hit%20Result%20Structure%20%28by%20ref%29))
  (Development|PrintString (Utilities|String|Append "Enemy shot " (Utilities|GetDisplayName OtherComp)) true true "(R=0.602283,G=0.835775,B=1.000000,A=1.000000)")
  (Utilities|FlowControl|Delay 0.0)
  (Actor|DestroyActor))

(fn ConstructionScript)