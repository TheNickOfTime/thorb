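; Player character component that manages level streaming, combat enemy layouts, the bullet-hell minigame and background music.
; It binds to FPS-Character events, queuing level-set loads and unloads that Tick processes one at a time.
; Each combat space streams a random enemy sublevel; clearing it makes the minigame available, and losing the minigame rolls a different one.
; Loading or unloading the minigame swaps possession between player and bullet-hell character.
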(event Custom|OnReturnToMainMenu
  ;[1 1 1] Binding Events - Main Game
  (Default|CallUnloadMinigameLevel (Variables|Default|GetPlayer))
  (Class|GameplayStatics|UnloadStreamLevelbySoftObjectPtr (Variables|Default|GetCurrentEnemiesLevel) false)
  (Utilities|UnloadAllLoadedLevels
    (:out
      ;;[1 1 1] Attn Mika
      (CallFunction|PickNewBGMusic "NewEnumerator6")
      (CallFunction|StartBGMusic 0.0 1.0 0.0 "Linear"))))

(event Custom|LoadMinigame
  (params (MinigameVersion :type Integer))
  ;[1 1 1] Binding Events - Minigame-Related
  (Utilities|OnLoadMinigame MinigameVersion) ; Attn Mika
  (Default|CallSetMinigameViewon (Variables|Default|GetPlayer)))

(event Custom|UnloadMinigame
  ;[1 1 1] Binding Events - Minigame-Related
  (Default|CallSetMinigameViewOff (Variables|Default|GetPlayer))
  (Utilities|OnUnloadMinigame) ; Attn Mika
)

(event Custom|OnBeginNewCombatSpace
  (params (Level :type LevelSet%20Enum :default "NewEnumerator0"))
  ;[1 1 1] Binding Events - Main Game
  (CallFunction|AssignEnemiesLevelSet Level)
  ;;[1 1 1] Attn Mika
  (Utilities|LoadRandomEnemyLevel))

(event Custom|OnWinMinigame
  ;[1 1 1] Binding Events - Minigame-Related
  (Variables|Default|SetPreviousEnemyLevelIndex -1))

(event Custom|OnLoadingLevel
  (params (LevelToLoad :type LevelSet%20Enum :default "NewEnumerator0"))
  ;[1 1 1] Binding Events - Main Game
  (Utilities|LoadLevelSet LevelToLoad))

(event Custom|OnUnloadingLevel
  (params (LevelToUnload :type LevelSet%20Enum :default "NewEnumerator0"))
  ;[1 1 1] Binding Events - Main Game
  (Utilities|UnloadLevelSet LevelToUnload))

(event Custom|OnLoseMinigame
  ;[1 1 1] Binding Events - Minigame-Related
  (Utilities|LoadRandomEnemyLevel))

(event Custom|OnMakeMinigameAvailable
  ;[1 1 1] Binding Events - Minigame-Related
  ;[1 1 1] Attn Mika
  (CallFunction|EndBGMusic 2.0 0.0 "Linear")
  (Class|GameplayStatics|UnloadStreamLevelbySoftObjectPtr (Variables|Default|GetCurrentEnemiesLevel) false))

(event Custom|OnEnemyDeath
  ;[1 1 1] Binding Events - Main Game
  (bind _result (Math|Integer|DecrementInt (Variables|Default|GetRemainingEnemies))
    (:%20%20
      (if (<= _result 0)
        (Default|CallMakeMinigameAvailable (Variables|Default|GetPlayer))))))

(event EventBeginPlay
  (Utilities|FlowControl|Sequence
    (:then_0
      ;[1 1 1] Getting References
      (bind _asfps_character (Utilities|Casting|CastToFPS-Character (Components|GetOwner)))
      (Variables|Default|SetPlayer _asfps_character)
      (bind _asfps_controller (Utilities|Casting|CastToFPS-Controller (Game|GetPlayerController 0)))
      (Variables|Default|SetControllerRef _asfps_controller)
      ;[1 1 1] Attn Mika
      (CallFunction|PickNewBGMusic "NewEnumerator6")
      (CallFunction|StartBGMusic 0.5 0.4 0.0 "Linear"))
    (:then_1
      ;[1 1 1] Binding Events - Minigame-Related
      (EventDispatchers|BindEventtoLoadMinigameLevel (Variables|Default|GetPlayer) (delegate Custom|LoadMinigame))
      (EventDispatchers|BindEventtoUnloadMinigameLevel (Variables|Default|GetPlayer) (delegate Custom|UnloadMinigame)))
    (:then_2
      (EventDispatchers|BindEventtoWinMinigame (Variables|Default|GetPlayer) (delegate Custom|OnWinMinigame))
      (EventDispatchers|BindEventtoLoseMinigame (Variables|Default|GetPlayer) (delegate Custom|OnLoseMinigame))
      (EventDispatchers|BindEventtoMakeMinigameAvailable (Variables|Default|GetPlayer) (delegate Custom|OnMakeMinigameAvailable)))
    (:then_3
      ;[1 1 1] Binding Events - Main Game
      (EventDispatchers|BindEventtoLoadLevel (Variables|Default|GetPlayer) (delegate Custom|OnLoadingLevel))
      (EventDispatchers|BindEventtoUnloadLevel (Variables|Default|GetPlayer) (delegate Custom|OnUnloadingLevel))
      (EventDispatchers|BindEventtoBeginNewCombatSpace (Variables|Default|GetPlayer) (delegate Custom|OnBeginNewCombatSpace))
      (EventDispatchers|BindEventtoEnemyDeath (Variables|Default|GetPlayer) (delegate Custom|OnEnemyDeath)))
    (:then_4
      (EventDispatchers|BindEventtoReturntoMainMenu (Variables|Default|GetPlayer) (delegate Custom|OnReturnToMainMenu)))
    (:then_5
      ;[1 1 1] Initializing Levels
      (CallFunction|InitializeLevelSets))))

(event EventTick
  (params (DeltaSeconds :type Float%20%28single-precision%29))
  ;[1 1 1] Load/Unload Levels
  (if (Utilities|CheckifLeveltoLoad)
    (Utilities|LoadFirstLevel)
    (elif (Utilities|CheckifLeveltoUnload)
      (Utilities|UnloadFirstLevel))))

(fn InitializeMinigameVariables
  (params (MinigameVersion :type Integer))
  (Variables|Default|SetMinigameVersion MinigameVersion))

(fn ClearMinigameVariables)

(fn InitializeLevelSets
  (bind _interior_03b_enemies_set (Variables|LevelSets|Getinterior-03b-Enemies-Set))
  (bind _interior_05a_enemies_set (Variables|LevelSets|Getinterior-05a-Enemies-Set))
  (bind _interior_05b_enemies_set (Variables|LevelSets|Getinterior-05b-Enemies-Set))
  (bind _interior_01a_enemies_set (Variables|LevelSets|Getinterior-01a-Enemies-Set))
  (bind _interior_01b_enemies_set (Variables|LevelSets|Getinterior-01b-Enemies-Set))
  (bind _interior_03a_enemies_set (Variables|LevelSets|Getinterior-03a-Enemies-Set))
  (Utilities|Array|Add (Variables|LevelSets|Getinterior-01a-Set) (Variables|Levels|Getinterior-01a))
  (Utilities|Array|Add _interior_01a_enemies_set (Variables|Levels|Getinterior-01a-enemies-01))
  (Utilities|Array|Add _interior_01a_enemies_set (Variables|Levels|Getinterior-01a-enemies-02))
  (Utilities|Array|Add _interior_01a_enemies_set (Variables|Levels|Getinterior-01a-enemies-03))
  (Utilities|Array|Add _interior_01a_enemies_set (Variables|Levels|Getinterior-01a-enemies-04))
  (Utilities|Array|Add _interior_01a_enemies_set (Variables|Levels|Getinterior-01a-enemies-05))
  (Utilities|Array|Add _interior_01a_enemies_set (Variables|Levels|Getinterior-01a-enemies-06))
  (Utilities|Array|Add (Variables|LevelSets|Getinterior-01b-Set) (Variables|Levels|Getinterior-01b))
  (Utilities|Array|Add _interior_01b_enemies_set (Variables|Levels|Getinterior-01b-enemies-01))
  (Utilities|Array|Add _interior_01b_enemies_set (Variables|Levels|Getinterior-01b-enemies-02))
  (Utilities|Array|Add _interior_01b_enemies_set (Variables|Levels|Getinterior-01b-enemies-03))
  (Utilities|Array|Add _interior_01b_enemies_set (Variables|Levels|Getinterior-01b-enemies-04))
  (Utilities|Array|Add _interior_01b_enemies_set (Variables|Levels|Getinterior-01b-enemies-05))
  (Utilities|Array|Add _interior_01b_enemies_set (Variables|Levels|Getinterior-01b-enemies-06))
  (Utilities|Array|Add (Variables|LevelSets|Getexterior-01-Set) (Variables|Levels|Getexterior-01))
  (Utilities|Array|Add (Variables|LevelSets|Getinterior-03a-Set) (Variables|Levels|Getinterior-03a))
  (Utilities|Array|Add _interior_03a_enemies_set (Variables|Levels|Getinterior-03a-enemies-01))
  (Utilities|Array|Add _interior_03a_enemies_set (Variables|Levels|Getinterior-03a-enemies-02))
  (Utilities|Array|Add _interior_03a_enemies_set (Variables|Levels|Getinterior-03a-enemies-03))
  (Utilities|Array|Add _interior_03a_enemies_set (Variables|Levels|Getinterior-03a-enemies-04))
  (Utilities|Array|Add _interior_03a_enemies_set (Variables|Levels|Getinterior-03a-enemies-05))
  (Utilities|Array|Add _interior_03a_enemies_set (Variables|Levels|Getinterior-03a-enemies-06))
  (Utilities|Array|Add (Variables|LevelSets|Getinterior-03b-Set) (Variables|Levels|Getinterior-03b))
  (Utilities|Array|Add _interior_03b_enemies_set (Variables|Levels|Getinterior-03b-enemies-01))
  (Utilities|Array|Add _interior_03b_enemies_set (Variables|Levels|Getinterior-03b-enemies-02))
  (Utilities|Array|Add _interior_03b_enemies_set (Variables|Levels|Getinterior-03b-enemies-03))
  (Utilities|Array|Add _interior_03b_enemies_set (Variables|Levels|Getinterior-03b-enemies-04))
  (Utilities|Array|Add _interior_03b_enemies_set (Variables|Levels|Getinterior-03b-enemies-05))
  (Utilities|Array|Add _interior_03b_enemies_set (Variables|Levels|Getinterior-03b-enemies-06))
  (Utilities|Array|Add (Variables|LevelSets|Getexterior-02-Set) (Variables|Levels|Getexterior-02))
  (Utilities|Array|Add (Variables|LevelSets|Getinterior-05a-Set) (Variables|Levels|Getinterior-05a))
  (Utilities|Array|Add _interior_05a_enemies_set (Variables|Levels|Getinterior-05a-enemies-01))
  (Utilities|Array|Add _interior_05a_enemies_set (Variables|Levels|Getinterior-05a-enemies-02))
  (Utilities|Array|Add _interior_05a_enemies_set (Variables|Levels|Getinterior-05a-enemies-03))
  (Utilities|Array|Add _interior_05a_enemies_set (Variables|Levels|Getinterior-05a-enemies-04))
  (Utilities|Array|Add _interior_05a_enemies_set (Variables|Levels|Getinterior-05a-enemies-05))
  (Utilities|Array|Add _interior_05a_enemies_set (Variables|Levels|Getinterior-05a-enemies-06))
  (Utilities|Array|Add (Variables|LevelSets|Getinterior-05b-Set) (Variables|Levels|Getinterior-05b))
  (Utilities|Array|Add _interior_05b_enemies_set (Variables|Levels|Getinterior-05b-enemies-01))
  (Utilities|Array|Add _interior_05b_enemies_set (Variables|Levels|Getinterior-05b-enemies-02))
  (Utilities|Array|Add _interior_05b_enemies_set (Variables|Levels|Getinterior-05b-enemies-03))
  (Utilities|Array|Add _interior_05b_enemies_set (Variables|Levels|Getinterior-05b-enemies-04))
  (Utilities|Array|Add _interior_05b_enemies_set (Variables|Levels|Getinterior-05b-enemies-05))
  (Utilities|Array|Add _interior_05b_enemies_set (Variables|Levels|Getinterior-05b-enemies-06)))

(fn AssignEnemiesLevelSet
  (params (Level :type LevelSet%20Enum :default "NewEnumerator0"))
  (Variables|Default|SetCurrentBGMusic Level)
  (Variables|Default|SetCurrentEnemiesLevelSet (Utilities|Select :Index Level :NewEnumerator0 (Variables|LevelSets|Getinterior-01a-Enemies-Set) :NewEnumerator1 (Variables|LevelSets|Getinterior-01b-Enemies-Set) :NewEnumerator2 0 :NewEnumerator3 (Variables|LevelSets|Getinterior-03a-Enemies-Set) :NewEnumerator7 (Variables|LevelSets|Getinterior-03b-Enemies-Set) :NewEnumerator4 0 :NewEnumerator5 (Variables|LevelSets|Getinterior-05a-Enemies-Set) :NewEnumerator8 (Variables|LevelSets|Getinterior-05b-Enemies-Set) :NewEnumerator6 0 :NewEnumerator9 0))
  (CallFunction|PickNewBGMusic Level))

(fn GetNumberOfEnemies
  (bind _outactors (Actor|GetAllActorsOfClass "/Game/Blueprints/AI/Enemy-Character.Enemy-Character_C"))
  (Variables|Default|SetRemainingEnemies (Utilities|Array|Length _outactors))
  (Development|PrintString (Utilities|String|ToString(Integer) (Utilities|Array|Length _outactors))))

(fn PickNewBGMusic
  (params (Level :type LevelSet%20Enum :default "NewEnumerator0"))
  (bind _player (Variables|Default|GetPlayer))
  (CallFunction|EndBGMusic 0.0 0.0 "Linear")
  (Variables|Default|SetBG_Music (Utilities|Select :Index Level :NewEnumerator0 (Variables|/Game/Blueprints/Player/FPS-Character.FPS-Character_C|GetMUS_interior-1a _player) :NewEnumerator1 (Variables|/Game/Blueprints/Player/FPS-Character.FPS-Character_C|GetMUS_interior-1b _player) :NewEnumerator2 0 :NewEnumerator3 (Variables|/Game/Blueprints/Player/FPS-Character.FPS-Character_C|GetMUS_interior-3a _player) :NewEnumerator7 (Variables|/Game/Blueprints/Player/FPS-Character.FPS-Character_C|GetMUS_interior-3b _player) :NewEnumerator4 0 :NewEnumerator5 (Variables|/Game/Blueprints/Player/FPS-Character.FPS-Character_C|GetMUS_interior-5a _player) :NewEnumerator8 (Variables|/Game/Blueprints/Player/FPS-Character.FPS-Character_C|GetMUS_interior-5b _player) :NewEnumerator6 (Variables|/Game/Blueprints/Player/FPS-Character.FPS-Character_C|GetMUS_main_menu _player) :NewEnumerator9 (Variables|/Game/Blueprints/Player/FPS-Character.FPS-Character_C|GetMUS_minigame _player))))

(fn StartBGMusic
  (params (Fade%20in%20Duration :type Float%20%28single-precision%29) (Fade%20Volume%20Level :type Float%20%28single-precision%29) (StartTime :type Float%20%28single-precision%29) (FadeCurve :type EAudioFaderCurve%20Enum :default "Linear"))
  (bind _bg_music (Variables|Default|GetBG_Music))
  (Utilities|IsValid _bg_music
    (:Is%20Valid
      (Audio|Components|Audio|FadeIn _bg_music Fade%20in%20Duration Fade%20Volume%20Level StartTime FadeCurve :!class /Script/Engine.AudioComponent))))

(fn EndBGMusic
  (params (Fade%20Out%20Duration :type Float%20%28single-precision%29) (Fade%20Volume%20Level :type Float%20%28single-precision%29) (FadeCurve :type EAudioFaderCurve%20Enum :default "Linear"))
  (bind _bg_music (Variables|Default|GetBG_Music))
  (Utilities|IsValid _bg_music
    (:Is%20Valid
      (Audio|Components|Audio|FadeOut _bg_music Fade%20Out%20Duration Fade%20Volume%20Level FadeCurve :!class /Script/Engine.AudioComponent))))