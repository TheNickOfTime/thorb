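; Test player controller for switching possession between two pawns.
; On BeginPlay it stores the player pawn as Pawn1 and sets it as the view target.
; Enter spawns a TestPawn2 at a fixed location if Pawn2 is unset.
; Space alternates possession through a FlipFlop, prints the current pawn's name, then resets the view target to Pawn1, so the camera stays there.
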(event EventBeginPlay
  (bind _output_get (Variables|Default|SetPawn1 (.AsTest%20Pawn%201 (Utilities|Casting|CastToTestPawn1 (Game|Player|GetPlayerPawn 0)))))
  (Game|Player|SetViewTargetwithBlend _output_get 0.0 "VTBlend_Linear" 0.0 false))

(event Input|KeyboardEvents|SpaceBar
  (params (Key :type Key%20Structure :default "None"))
  (:Pressed
    (Utilities|FlowControl|FlipFlop
      (:A
        (Pawn|Possess (Variables|Default|GetPawn2)))
      (:B
        (Pawn|Possess (Variables|Default|GetPawn1))))
    (Development|PrintString (Utilities|GetDisplayName (Game|Player|GetPlayerPawn 0)))
    (Game|Player|SetViewTargetwithBlend (stale EventBeginPlay _output_get) 0.0 "VTBlend_Linear" 0.0 false)))

(event Input|KeyboardEvents|Enter
  (params (Key :type Key%20Structure :default "None"))
  (:Pressed
    (if (== (Variables|Default|GetPawn2) 0)
      (bind _returnvalue (Game|SpawnActorfromClass "/Game/Test/Nick/Blueprints/TestPawn2.TestPawn2_C" (Math|Transform|MakeTransform "0,250.000000,100.000000") "Undefined" 0 0))
      (Variables|Default|SetPawn2 _returnvalue)
      (Development|PrintString "Spawn Pawn 2"))))

(fn ConstructionScript)